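; Moving platform that makes the player slide by removing ground friction while they overlap its Box.
; After a start delay, a timeline lerps the platform between StartLoc and EndLoc, alternating direction after a pause at each end.
; On overlap it caches BP_PlayerBase's friction and braking values and zeroes them.
; On exit it restores that cache only if the player overlaps no other BP_platform_black.
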(event OnComponentBeginOverlap(Box)
  (params (OverlappedComponent :type Primitive%20Component%20Object%20Reference) (OtherActor :type Actor%20Object%20Reference) (OtherComp :type Primitive%20Component%20Object%20Reference) (OtherBodyIndex :type Integer) (bFromSweep :type Boolean) (SweepResult :type Hit%20Result%20Structure%20%28by%20ref%29))
  (bind _asbp_player_base (Utilities|Casting|CastToBP_PlayerBase OtherActor))
  (CallFunction|BreakFriction _asbp_player_base))

(event OnComponentEndOverlap(Box)
  (params (OverlappedComponent :type Primitive%20Component%20Object%20Reference) (OtherActor :type Actor%20Object%20Reference) (OtherComp :type Primitive%20Component%20Object%20Reference) (OtherBodyIndex :type Integer))
  (bind _asbp_player_base (Utilities|Casting|CastToBP_PlayerBase OtherActor))
  (if (== (Utilities|Array|Length (Collision|GetOverlappingActors _asbp_player_base "BP_platform_black_C" :!class /Script/Engine.Actor)) 0)
    (CallFunction|ResumeFriction _asbp_player_base)))

(event EventBeginPlay
  (Utilities|FlowControl|Delay (Variables|Movement|GetStartDelay))
  (Variables|Movement|SetStartLoc (Transformation|GetWorldLocation (Variables|Default|GetPlatform)))
  (Components|Timeline|SetPlayRate (Variables|Default|GetMovement) (Variables|Movement|GetTranslationRate))
  (bind _newtrack_2 (Timeline|Movement PlayFromStart)
    (:Update
      (Transformation|SetRelativeLocation (Variables|Default|GetPlatform) (Math|Vector|Lerp(Vector) (Variables|Movement|GetStartLoc) (Variables|Movement|GetEndLoc) _newtrack_2) false false))
    (:Finished
      (Utilities|FlowControl|Delay (Variables|Movement|GetDelay))
      (if (Variables|Movement|GetIsLooped)
        (Variables|Movement|SetIsLooped false)
        (Timeline|Movement PlayFromStart)
        (else
          (Variables|Movement|SetIsLooped true)
          (Timeline|Movement ReverseFromEnd))))))

(event EventTick
  (params (DeltaSeconds :type Float%20%28single-precision%29)))

(fn ConstructionScript)

(fn ResumeFriction
  (params (Player_ref :type BP%20Player%20Base%20Object%20Reference))
  (bind _charactermovement (Variables|/Script/Engine.Character|GetCharacterMovement Player_ref))
  (Variables|/Script/Engine.CharacterMovementComponent|SetBrakingFriction _charactermovement (Variables|Default|Getdefault_breaking))
  (Variables|/Script/Engine.CharacterMovementComponent|SetBrakingDecelerationWalking _charactermovement (Variables|Default|Getdefault_deceleration))
  (Variables|/Script/Engine.CharacterMovementComponent|SetGroundFriction _charactermovement (Variables|Default|GetDefault_Friction))
  (return))

(fn BreakFriction
  (params (player_ref :type BP%20Player%20Base%20Object%20Reference))
  (bind _charactermovement (Variables|/Script/Engine.Character|GetCharacterMovement player_ref))
  (Variables|Default|Setdefault_breaking (Variables|/Script/Engine.CharacterMovementComponent|GetBrakingFriction _charactermovement))
  (Variables|Default|Setdefault_deceleration (Variables|/Script/Engine.CharacterMovementComponent|GetBrakingDecelerationWalking _charactermovement))
  (Variables|Default|SetDefault_Friction (Variables|/Script/Engine.CharacterMovementComponent|GetGroundFriction _charactermovement))
  (Variables|/Script/Engine.CharacterMovementComponent|SetGroundFriction _charactermovement 0.0)
  (Variables|/Script/Engine.CharacterMovementComponent|SetBrakingFriction _charactermovement 0.0)
  (Variables|/Script/Engine.CharacterMovementComponent|SetBrakingDecelerationWalking _charactermovement 0.0)
  (return))