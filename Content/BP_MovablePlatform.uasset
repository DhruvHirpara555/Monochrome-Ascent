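; Moving platform actor that travels back and forth between its start position and EndLoc indefinitely.
; After a start delay, it captures the Platform's world location and plays the Movement timeline at TranslationRate.
; The timeline lerps between the two points, writing the result as a relative location without sweep.
; Each finish waits a delay, then IsLooped toggles to choose forward or reverse playback.
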(event EventBeginPlay
  (Utilities|FlowControl|Delay (Variables|Movement|GetStartDelay))
  (Variables|Movement|SetStartLoc (Transformation|GetWorldLocation (Variables|Default|GetPlatform)))
  (Components|Timeline|SetPlayRate (Variables|Default|GetMovement) (Variables|Movement|GetTranslationRate))
  (bind _newtrack_2 (Timeline|Movement PlayFromStart)
    (:Update
      (Transformation|SetRelativeLocation (Variables|Default|GetPlatform) (Math|Vector|Lerp(Vector) (Variables|Movement|GetStartLoc) (Variables|Movement|GetEndLoc) _newtrack_2) false false))
    (:Finished
      (Utilities|FlowControl|Delay (Variables|Movement|GetDelay))
      (if (Variables|Movement|GetIsLooped)
        (Variables|Movement|SetIsLooped false)
        (Timeline|Movement PlayFromStart)
        (else
          (Variables|Movement|SetIsLooped true)
          (Timeline|Movement ReverseFromEnd))))))

(event EventTick
  (params (DeltaSeconds :type Float%20%28single-precision%29)))

(fn ConstructionScript)