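; BP_movable_black is a moving platform that travels back and forth endlessly between its starting location and EndLoc.
; After a start delay, the Movement timeline lerps the platform's relative location from a captured world-space start, pausing before each reversal via the IsLooped toggle.
; A Box overlap with BP_PlayerBase calls BreakFriction, but both friction functions are empty and ResumeFriction is never called.
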(event OnComponentEndOverlap(Box)
  (params (OverlappedComponent :type Primitive%20Component%20Object%20Reference) (OtherActor :type Actor%20Object%20Reference) (OtherComp :type Primitive%20Component%20Object%20Reference) (OtherBodyIndex :type Integer))
  (bind _asbp_player_base (Utilities|Casting|CastToBP_PlayerBase OtherActor)))

(event OnComponentBeginOverlap(Box)
  (params (OverlappedComponent :type Primitive%20Component%20Object%20Reference) (OtherActor :type Actor%20Object%20Reference) (OtherComp :type Primitive%20Component%20Object%20Reference) (OtherBodyIndex :type Integer) (bFromSweep :type Boolean) (SweepResult :type Hit%20Result%20Structure%20%28by%20ref%29))
  (bind _asbp_player_base (Utilities|Casting|CastToBP_PlayerBase OtherActor))
  (CallFunction|BreakFriction _asbp_player_base))

(event EventBeginPlay
  (Utilities|FlowControl|Delay (Variables|Movement|GetStartDelay))
  (Variables|Movement|SetStartLoc (Transformation|GetWorldLocation (Variables|Default|GetPlatform)))
  (Components|Timeline|SetPlayRate (Variables|Default|GetMovement) (Variables|Movement|GetTranslationRate))
  (bind _newtrack_2 (Timeline|Movement PlayFromStart)
    (:Update
      (Transformation|SetRelativeLocation (Variables|Default|GetPlatform) (Math|Vector|Lerp(Vector) (Variables|Movement|GetStartLoc) (Variables|Movement|GetEndLoc) _newtrack_2) false false))
    (:Finished
      (Utilities|FlowControl|Delay (Variables|Movement|GetDelay))
      (if (Variables|Movement|GetIsLooped)
        (Variables|Movement|SetIsLooped false)
        (Timeline|Movement PlayFromStart)
        (else
          (Variables|Movement|SetIsLooped true)
          (Timeline|Movement ReverseFromEnd))))))

(event EventTick
  (params (DeltaSeconds :type Float%20%28single-precision%29)))

(fn ConstructionScript)

(fn BreakFriction
  (params (player_ref :type BP%20Player%20Base%20Object%20Reference)))

(fn ResumeFriction
  (params (Player_ref :type BP%20Player%20Base%20Object%20Reference)))