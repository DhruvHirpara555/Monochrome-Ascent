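; Spinning platform actor that rotates its Platform component every tick by a rotation rate scaled by delta time.
; Two helper functions cache and zero a player's ground friction, braking friction and walking deceleration, then restore them.
; Capsule overlap events cast to BP_PlayerBase but do nothing further, so neither friction helper is called in this graph.
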(event OnComponentBeginOverlap(Capsule)
  (params (OverlappedComponent :type Primitive%20Component%20Object%20Reference) (OtherActor :type Actor%20Object%20Reference) (OtherComp :type Primitive%20Component%20Object%20Reference) (OtherBodyIndex :type Integer) (bFromSweep :type Boolean) (SweepResult :type Hit%20Result%20Structure%20%28by%20ref%29))
  (Utilities|Casting|CastToBP_PlayerBase OtherActor))

(event OnComponentEndOverlap(Capsule)
  (params (OverlappedComponent :type Primitive%20Component%20Object%20Reference) (OtherActor :type Actor%20Object%20Reference) (OtherComp :type Primitive%20Component%20Object%20Reference) (OtherBodyIndex :type Integer))
  (bind _asbp_player_base (Utilities|Casting|CastToBP_PlayerBase OtherActor)))

(event EventBeginPlay)

(event EventTick
  (params (DeltaSeconds :type Float%20%28single-precision%29))
  (bind _platform (Variables|Default|GetPlatform))
  (bind _output_get (Variables|Default|SetRotationStart (Variables|/Script/Engine.SceneComponent|GetRelativeRotation _platform)))
  (Transformation|SetRelativeRotation _platform (Math|Rotator|CombineRotators _output_get (* (Variables|Default|GetRotRate) DeltaSeconds)) false false))

(fn ConstructionScript)

(fn ResumeFriction
  (params (Player_ref :type BP%20Player%20Base%20Object%20Reference))
  (bind _charactermovement (Variables|/Script/Engine.Character|GetCharacterMovement Player_ref))
  (Variables|/Script/Engine.CharacterMovementComponent|SetBrakingFriction _charactermovement (Variables|Default|Getdefault_breaking))
  (Variables|/Script/Engine.CharacterMovementComponent|SetBrakingDecelerationWalking _charactermovement (Variables|Default|Getdefault_deceleration))
  (Variables|/Script/Engine.CharacterMovementComponent|SetGroundFriction _charactermovement (Variables|Default|GetDefault_Friction))
  (return))

(fn BreakFriction
  (params (player_ref :type BP%20Player%20Base%20Object%20Reference))
  (bind _charactermovement (Variables|/Script/Engine.Character|GetCharacterMovement player_ref))
  (Variables|Default|Setdefault_breaking (Variables|/Script/Engine.CharacterMovementComponent|GetBrakingFriction _charactermovement))
  (Variables|Default|Setdefault_deceleration (Variables|/Script/Engine.CharacterMovementComponent|GetBrakingDecelerationWalking _charactermovement))
  (Variables|Default|SetDefault_Friction (Variables|/Script/Engine.CharacterMovementComponent|GetGroundFriction _charactermovement))
  (Variables|/Script/Engine.CharacterMovementComponent|SetGroundFriction _charactermovement 0.0)
  (Variables|/Script/Engine.CharacterMovementComponent|SetBrakingFriction _charactermovement 0.0)
  (Variables|/Script/Engine.CharacterMovementComponent|SetBrakingDecelerationWalking _charactermovement 0.0)
  (return))