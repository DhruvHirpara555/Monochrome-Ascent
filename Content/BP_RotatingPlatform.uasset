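; BP_RotatingPlatform is a platform that swings back and forth between its starting rotation and RotationEnd.
; On BeginPlay it captures Platform's world rotation and plays a timeline at RotationSpeed, lerping Root's relative rotation.
; A Delay chained from the timeline's Update, not Finished, toggles IsLooped to alternate PlayFromStart and ReverseFromEnd.
; The construction script stores Platform's relative transform, which the event graph never reads.
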(event EventBeginPlay
  (Variables|Default|SetRotationStart (Transformation|GetWorldRotation (Variables|Default|GetPlatform)))
  (Components|Timeline|SetPlayRate (Variables|Default|GetRotTimeline) (Variables|Default|GetRotationSpeed))
  (bind _newtrack_0 (Timeline|RotTimeline PlayFromStart)
    (:Update
      (Transformation|SetRelativeRotation (Variables|Default|Getroot) (Math|Rotator|Lerp(Rotator) (Variables|Default|GetRotationStart) (Variables|Default|GetRotationEnd) _newtrack_0) false false)
      (Utilities|FlowControl|Delay (Variables|Default|GetDelay))
      (if (Variables|Default|GetIsLooped)
        (Variables|Default|SetIsLooped false)
        (Timeline|RotTimeline PlayFromStart)
        (else
          (Variables|Default|SetIsLooped true)
          (Timeline|RotTimeline ReverseFromEnd))))))

(fn ConstructionScript
  (Variables|Default|SetRelTransform (Transformation|GetRelativeTransform (Variables|Default|GetPlatform))))